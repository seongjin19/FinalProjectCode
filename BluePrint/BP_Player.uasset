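; BP_Player is the player character, with a hitscan weapon for fighting BP_Monster bosses.
; FireWeapon plays the fire montage, then line-traces from a screen point slightly above centre, spawning an explosion at hits and playing its sound at world origin.
; Monster hits subtract BossHP directly and call MonsterDeath at zero.
; BeginPlay caches BP_PlayerStat, but Tick's HP check does nothing; DestroyActor and a muzzle-socket trace are unwired.
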(event `self.ReceiveBeginPlay`
  (bind _asbp_player_stat (cast `/Game/BluePrint/BP_PlayerStat` (`GameplayStatics.GetPlayerState` 0)))
  (set `self.As BP Player Stat` _asbp_player_stat))

(event `self.ReceiveTick`
  (params (DeltaSeconds :type "Float (single-precision)"))
  (if (<= (`/Game/BluePrint/BP_PlayerStat.HP` (`self.As BP Player Stat`)) 0.0)
    _))

(fn `FireWeapon`
  (bind (_returnvalue_x _returnvalue_y) (`KismetMathLibrary.BreakVector2D` (`WidgetLayoutLibrary.GetViewportSize`)))
  (bind (_worldposition _worlddirection _returnvalue) (`GameplayStatics.DeprojectScreenToWorld` (`GameplayStatics.GetPlayerController` 0) (`KismetMathLibrary.MakeVector2D` (/ _returnvalue_x 2.0) (- (/ _returnvalue_y 2.0) 50.0))))
  (`self.PlayAnimMontage` "/Game/Animation/AM_Fire.AM_Fire" 1.0 "start")
  (if _returnvalue
    (bind _outhit (`KismetSystemLibrary.LineTraceSingle` :`Start` _worldposition :`End` (+ _worldposition (* _worlddirection 5000.0)) :`TraceChannel` "TraceTypeQuery3" :`DrawTime` 1.0))
    (bind (_bblockinghit _binitialoverlap _time _distance _location _impactpoint _normal _impactnormal _physmat _hitactor) (`GameplayStatics.BreakHitResult` _outhit))
    (if _bblockinghit
      (set `self.Hit Actor` _hitactor)
      (`GameplayStatics.SpawnEmitterAtLocation` "/Game/StarterContent/Particles/P_Explosion.P_Explosion" _location)
      (`GameplayStatics.PlaySoundAtLocation` "/Game/StarterContent/Audio/Explosion01.Explosion01" (0.0 0.0 0.0) (struct) 1.0 1.0 0.0 null null null null)
      (bind _asbp_monster (cast `/Game/BluePrint/BP_Monster` (`self.Hit Actor`)))
      (set `self.As BP Monster` _asbp_monster)
      (bind _output_get (set `/Game/BluePrint/BP_Monster.BossHP` (- (`/Game/BluePrint/BP_Monster.BossHP` (`self.As BP Monster`)) 2.0) (`self.As BP Monster`)))
      (if (<= _output_get 0.0)
        (`/Game/BluePrint/BP_Monster.Monster Death` (`self.As BP Monster`))))))

(fn `UserConstructionScript`)