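; Player controller that turns input into movement, mouse look and attacks for the player character.
; Move axes push player pawn 0 along the controller actor's own forward and right vectors, while Turn and LookUp feed yaw and pitch input.
; Pressing Fire casts player character 0 to BP_Player and calls its FireWeapon, leaving the weapon logic to that Blueprint.
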(event `InputAxis|MoveForward`
  (params (AxisValue :type "Float (single-precision)"))
  ;[1 1 1] 플레이어 이동
  (`Pawn.AddMovementInput` (`GameplayStatics.GetPlayerPawn` 0) (`self.GetActorForwardVector`) AxisValue false))

(event `InputAxis|MoveRight`
  (params (AxisValue :type "Float (single-precision)"))
  ;[1 1 1] 플레이어 이동
  (`Pawn.AddMovementInput` (`GameplayStatics.GetPlayerPawn` 0) (`self.GetActorRightVector`) AxisValue false))

(event `InputAxis|Turn`
  (params (AxisValue :type "Float (single-precision)"))
  ;[1 1 1] 마우스 시점이동
  (`self.AddYawInput` AxisValue))

(event `InputAxis|LookUp`
  (params (AxisValue :type "Float (single-precision)"))
  ;[1 1 1] 마우스 시점이동
  (`self.AddPitchInput` AxisValue))

(event `InputAction|Fire`
  (params (Key :type "Key Structure"))
  ;[1 1 1] 공격
  (:`Pressed`
    (bind _asbp_player (cast `/Game/BluePrint/BP_Player` (`GameplayStatics.GetPlayerCharacter` 0)))
    (`/Game/BluePrint/BP_Player.FireWeapon` _asbp_player)))

(fn `UserConstructionScript`)