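; Boss monster that attacks the player and whose death leads to the game-clear screen.
; Attack turns it toward the BP_Player actor and plays a punch montage through ABP_Monster.
; Tick destroys the actor once BossHP runs out.
; A separate MonsterDeath event, not called here, shows the GameClear widget and switches to UI-only input with a cursor, using the controller from the PlayerState cached at BeginPlay.
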(event `self.ReceiveTick`
  (params (DeltaSeconds :type "Float (single-precision)"))
  (if (<= (`self.BossHP`) 0.0)
    (`self.K2_DestroyActor`)))

(event `self.ReceiveBeginPlay`
  (bind _asbp_player_stat (cast `/Game/BluePrint/BP_PlayerStat` (`GameplayStatics.GetPlayerState` 0)))
  (set `self.As BP Player Stat` _asbp_player_stat))

(event `Attack`
  (bind _returnvalue (`GameplayStatics.GetActorOfClass` "/Game/BluePrint/BP_Player.BP_Player_C"))
  (`self.K2_SetActorRotation` (`KismetMathLibrary.FindLookAtRotation` (`self.K2_GetActorLocation`) (`self.K2_GetActorLocation` _returnvalue)))
  (bind _asabp_monster (cast `/Game/Animation/ABP_Monster` (`SkeletalMeshComponent.GetAnimInstance` (`self.Mesh`))))
  (`AnimInstance.Montage_Play` _asabp_monster "/Game/Animation/Attack_Punch_01_Montage.Attack_Punch_01_Montage" 1.0 "MontageLength" 0.0 true))

(event `Monster Death`
  (bind _returnvalue (`PlayerState.GetPlayerController` (`self.As BP Player Stat`)))
  (bind _returnvalue_2 (`|CreateWidget` "/Game/UI/GameClear.GameClear_C"))
  (`UserWidget.AddToViewport` _returnvalue_2 0)
  (`WidgetBlueprintLibrary.SetInputMode_UIOnlyEx` _returnvalue _returnvalue_2)
  (set `PlayerController.bShowMouseCursor` true _returnvalue))

(fn `UserConstructionScript`)